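; Push-switch actor that slides two parts, LeftIn and RightIn, along a timeline when switched on.
; The timeline's vector track drives their relative locations, with Y negated for RightIn so they move mirror-image.
; Release stops the timeline in place; LeftColi overlap also stops it and spawns an explosion at the actor, while end overlap resumes it.
; Overlaps are unfiltered, as the character cast is unconnected.
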(event `self.ReceiveTick`
  (params (DeltaSeconds :type "Float (single-precision)")))

(event `/Game/01_BluePrints/BPI_Item.Onswitch`
  (bind (_direction `_새_트랙_0`) (`Timeline|큐브 움직임` :!label _label)
    (:`Update`
      (`SceneComponent.K2_SetRelativeLocation` (`self.LeftIn`) `_새_트랙_0` false false)
      (`SceneComponent.K2_SetRelativeLocation` (`self.RightIn`) (* `_새_트랙_0` (1.0 -1.0 1.0)) false false))))

(event `/Game/01_BluePrints/BPI_Item.OnRelesed`
  (goto _label :!via `Stop`))

(event `self.ReceiveBeginPlay`)

(event `self.LeftColi.OnComponentEndOverlap`
  (params (OverlappedComponent :type "PrimitiveComponent Object Reference") (OtherActor :type "Actor Object Reference") (OtherComp :type "PrimitiveComponent Object Reference") (OtherBodyIndex :type Integer))
  (goto _label))

(event `self.LeftColi.OnComponentBeginOverlap`
  (params (OverlappedComponent :type "PrimitiveComponent Object Reference") (OtherActor :type "Actor Object Reference") (OtherComp :type "PrimitiveComponent Object Reference") (OtherBodyIndex :type Integer) (bFromSweep :type Boolean) (SweepResult :type "HitResult Structure (by ref)"))
  (`GameplayStatics.SpawnEmitterAtLocation` "/Game/StarterContent/Particles/P_Explosion.P_Explosion" (`self.K2_GetActorLocation`))
  (goto _label :!via `Stop`))

(fn `UserConstructionScript`)